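; Base RPG player character built on Mover-style intent-driven movement, handling input for moving, looking and crouching.
; Move input becomes a world-axis intent vector sent to RequestMoveByIntent and zeroed on release, while look input drives controller yaw and pitch.
; On restart it resets the player's Enhanced Input mappings to the default context; Left Ctrl is a hard-wired hold-to-crouch key.
; Tick prints the current movement mode on screen for debugging.
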(event `EnhancedInput|/Game/AgeOfMonsters/Input/Actions/IA_Move`
  (params (ActionValue :type "Vector2D Structure") (ElapsedSeconds :type "Float (double-precision)") (TriggeredSeconds :type "Float (double-precision)") (InputAction :type "InputAction Object Reference" :default "/Game/AgeOfMonsters/Input/Actions/IA_Move.IA_Move"))
  (:`Triggered`
    (bind _output_get (set `self.World Direction Intent` (`KismetMathLibrary.MakeVector` ActionValue_X ActionValue_Y) :!label _label))
    (`self.RequestMoveByIntent` _output_get))
  (:`Ongoing`
    (goto _label))
  (:`Completed`
    (`self.RequestMoveByIntent` (0.0 0.0 0.0))))

(event `EnhancedInput|/Game/AgeOfMonsters/Input/Actions/IA_Look`
  (params (ActionValue :type "Vector2D Structure") (ElapsedSeconds :type "Float (double-precision)") (TriggeredSeconds :type "Float (double-precision)") (InputAction :type "InputAction Object Reference" :default "/Game/AgeOfMonsters/Input/Actions/IA_Look.IA_Look"))
  (bind (_x _y) (`KismetMathLibrary.BreakVector2D` ActionValue))
  (:`Triggered`
    (`self.AddControllerYawInput` _x)
    (`self.AddControllerPitchInput` _y)))

(event `self.ReceiveTick`
  (params (DeltaSeconds :type "Float (single-precision)"))
  (`KismetSystemLibrary.PrintString` (`KismetStringLibrary.Conv_NameToString` (`MoverComponent.GetMovementModeName` (`self.CharacterMotionComponent`))) true false (struct :`G` 0.66 :`B` 1.0 :`A` 1.0) 0.0))

(event `self.ReceiveRestarted`
  (bind _returnvalue (`self.GetController`))
  (`/Engine/EditorBlueprintResources/StandardMacros.IsValid` _returnvalue
    (:`Is Valid`
      (bind _asplayer_controller (cast `PlayerController` _returnvalue))
      (bind _returnvalue_2 (pcsubsystem `EnhancedInputLocalPlayerSubsystem` _asplayer_controller))
      (`/Engine/EditorBlueprintResources/StandardMacros.IsValid` _returnvalue_2
        (:`Is Valid`
          (`EnhancedInputSubsystemInterface.ClearAllMappings` _returnvalue_2)
          (`self.ApplyIMC` _asplayer_controller))))))

(event `Key|LeftControl`
  (params (Key :type "Key Structure"))
  (:`Pressed`
    (`self.TryCrouch`))
  (:`Released`
    (`self.TryUnCrouch`)))

(fn `ApplyIMC`
  (params (Controller :type "PlayerController Object Reference"))
  (`EnhancedInputSubsystemInterface.AddMappingContext` (pcsubsystem `EnhancedInputLocalPlayerSubsystem` Controller) "/Game/AgeOfMonsters/Input/IMC_Default.IMC_Default" 0 (struct)))

(fn `UserConstructionScript`)