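; A Mover movement mode for character climbing, apparently an early prototype.
; Each simulation tick overwrites the updated primitive's physics velocity with a tiny fixed upward value whenever the proposed move has any direction intent, or zero otherwise.
; The tick keeps the starting mode as next mode but returns a fresh sync state with no mode name.
; Move generation defers to the parent, and transform-based movement nodes are left unwired.
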(fn `GetMs`
  (params (SimulationTickParams :type "SimulationTickParams Structure (by ref)"))
  (returns (`Step Ms` :type "Float (single-precision)"))
  (return (`.StepMs` (break `MoverTimeStep` (`.TimeStep` (break `SimulationTickParams` SimulationTickParams))))))

(fn `K2_OnGenerateMove`
  (params (StartState :type "MoverTickStartData Structure (by ref)") (TimeStep :type "MoverTimeStep Structure (by ref)"))
  (returns (ReturnValue :type "ProposedMove Structure"))
  (bind _returnvalue (`parent.K2_OnGenerateMove` StartState TimeStep))
  (return _returnvalue))

(fn `K2_OnSimulationTick`
  (params (Params :type "SimulationTickParams Structure (by ref)"))
  (returns (ReturnValue :type "MoverTickEndData Structure"))
  (locals (DeltaSeconds :type "Float (single-precision)" :default 0.0))
  (bind (_updatedcomponent _updatedprimitive _movercomponent _startstate _timestep _proposedmove) (break `SimulationTickParams` Params))
  (set `local.DeltaSeconds` (`self.GetDeltaSecondsFromParams` Params))
  (if (!= (`.DirectionIntent` (break `ProposedMove` _proposedmove)) (0.0 0.0 0.0))
    (`PrimitiveComponent.SetPhysicsLinearVelocity` _updatedprimitive (0.0 0.0 1.0) false "None")
    (else
      (`PrimitiveComponent.SetPhysicsLinearVelocity` _updatedprimitive (0.0 0.0 0.0) false "None")))
  (return (make `MoverTickEndData` (make `MoverSyncState` "None") (struct) (make `MovementModeTickEndState` 0.0 (`.MovementMode` (break `MoverSyncState` (`.SyncState` (break `MoverTickStartData` _startstate))))))))